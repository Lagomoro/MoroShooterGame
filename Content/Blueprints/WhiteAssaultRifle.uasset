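; White assault rifle weapon Blueprint that supplies cosmetic fire and hit effects through parent-class events.
; Firing attaches a muzzle flash, launches an effect actor by physics velocity from the fire arrow, and plays sound and camera shake.
; After a delay it destroys the flash and the effect actor's root component, not the actor itself.
; Hits play sound and particles from GetHitEffect, which currently returns the same pair for every physical material.
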(event EventBeginPlay
  (|CallParentFunction))

(event Collision|EventActorBeginOverlap
  (params (OtherActor :type Actor%20Object%20Reference))
  (|CallParentFunction OtherActor))

(event EventMakeFireEffectBP
  (params (Fired :type Boolean))
  (bind _weaponbody (Variables|Default|GetWeaponBody))
  (bind _weaponfirearrow (Variables|Default|GetWeaponFireArrow))
  (bind _returnvalue (Transformation|GetWorldLocation _weaponbody))
  (if Fired
    (bind _returnvalue_2 (Effects|SpawnEmitterAttached "/Game/SciFiWeapLight/FX/Particles/P_AssaultRifle_MuzzleFlash_Light.P_AssaultRifle_MuzzleFlash_Light" _weaponfirearrow "None" "0, 0, 0" "0, 0, 0" "2.000000,2.000000,2.000000"))
    (bind _returnvalue_3 (Game|SpawnActorfromClass "/Game/Blueprints/WhiteAssaultRifleEffect.WhiteAssaultRifleEffect_C" (Transformation|GetWorldTransform _weaponfirearrow) "Undefined" 0 0))
    (Class|PrimitiveComponent|SetAllPhysicsLinearVelocity (Variables|/Game/Blueprints/WhiteAssaultRifleEffect.WhiteAssaultRifleEffect_C|GetBase _returnvalue_3) (* (Math|Vector|GetForwardVector _weaponfirearrow) 10000) false)
    (Audio|PlaySoundatLocation "/Game/SciFiWeapLight/Sound/Rifle/Wavs/Rifle_Fire01.Rifle_Fire01" _returnvalue "0, 0, 0" 1.0 1.0 0.0 0 0 0)
    (Camera|PlayWorldCameraShake "/Game/Blueprints/MoroCameraShake.MoroCameraShake_C" _returnvalue 0.0 5e+02 3.0)
    (Utilities|FlowControl|Delay 5.0)
    (Components|DestroyComponent _returnvalue_2)))

(event EventMakeHitEffectBP
  (params (HitPhysicalMaterial :type Physical%20Material%20Object%20Reference) (HitLocation :type Vector :default "0, 0, 0") (HitActor :type Actor%20Object%20Reference) (HitComponent :type Primitive%20Component%20Object%20Reference) (HitBoneName :type Name :default "None"))
  (bind (_partical _sound) (CallFunction|GetHitEffect HitPhysicalMaterial))
  (Audio|PlaySoundatLocation _sound HitLocation "0, 0, 0" 1.0 1.0 0.0 0 0 0)
  (Effects|SpawnEmitteratLocation _partical HitLocation))

(event EventTick
  (params (DeltaSeconds :type Float%20%28single-precision%29)))

(fn ConstructionScript)

(fn GetHitEffect
  (params (Material :type Object%20Object%20Reference))
  (return "/Game/InfinityBladeEffects/Effects/FX_Mobile/combat/P_Shout_00.P_Shout_00" "/Game/SciFiWeapLight/Sound/SniperRifle/SR_ImpactSurface_Cue.SR_ImpactSurface_Cue"))