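; Game state Blueprint that holds a countdown timer, tracked as remaining time against a total.
; Functions subtract a given amount from the remaining time, report it stopped at zero or below, force a stop with a negative value, or restore the total.
; A ResetTimerEvent event wraps the reset.
; RepNotify handlers for GameStartTimer and RandomTimerValue1 are empty.
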(event Custom|Reset%20Timer%20Event
  (CallFunction|ResetTimer))

(fn ConstructionScript)

(fn OnRepGameStartTimer)

(fn OnRepRandomTimerValue1)

(fn DecreaseTimer
  (params (DecreaseVolume :type Float%20%28single-precision%29))
  (Variables|Default|SetTimeRemain (- (Variables|Default|GetTimeRemain) DecreaseVolume)))

(fn IsTimerStopped
  (return (<= (Variables|Default|GetTimeRemain) 0.0)))

(fn StopTimer
  (Variables|Default|SetTimeRemain -1.0))

(fn ResetTimer
  (Variables|Default|SetTimeRemain (Variables|Default|GetTimeTotal)))