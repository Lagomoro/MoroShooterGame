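; BulletRPG is a rocket launcher projectile that explodes on hit.
; It also explodes from Tick when the physics velocity of its rocket ammo component drops to nearly zero.
; The explosion plays a sound, spawns a particle emitter, applies radial damage with falloff, then destroys the actor.
; An impulse that would oppose the rocket's velocity is left disconnected and never runs.
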(event Collision|EventHit
  (params (MyComp :type Primitive%20Component%20Object%20Reference) (Other :type Actor%20Object%20Reference) (OtherComp :type Primitive%20Component%20Object%20Reference) (bSelfMoved :type Boolean) (HitLocation :type Vector :default "0, 0, 0") (HitNormal :type Vector :default "0, 0, 0") (NormalImpulse :type Vector :default "0, 0, 0") (Hit :type Hit%20Result%20Structure%20%28by%20ref%29))
  (bind _white_rocketlauncher_ammo (Variables|Default|GetWhite_RocketLauncher_Ammo))
  (bind _returnvalue (Transformation|GetWorldLocation _white_rocketlauncher_ammo))
  (Audio|PlaySoundatLocation "/Game/SciFiWeapLight/Sound/RocketLauncher/RL_Explosion_Cue.RL_Explosion_Cue" _returnvalue "0, 0, 0" 1.0 1.0 0.0 0 0 0)
  (Effects|SpawnEmitteratLocation "/Game/SciFiWeapLight/FX/Particles/P_RocketLauncher_Explosion_Dark.P_RocketLauncher_Explosion_Dark" _returnvalue)
  (Class|GameplayStatics|ApplyRadialDamagewithFalloff 3e+02 0.0 _returnvalue 0.0 1e+03 1.0 0 0 0 0 "ECC_Visibility")
  (Actor|DestroyActor))

(event EventTick
  (params (DeltaSeconds :type Float%20%28single-precision%29))
  (bind _white_rocketlauncher_ammo (Variables|Default|GetWhite_RocketLauncher_Ammo))
  (bind _returnvalue (Transformation|GetWorldLocation _white_rocketlauncher_ammo))
  (bind _returnvalue_2 (Physics|GetPhysicsLinearVelocity (Variables|Default|GetWhite_RocketLauncher_Ammo) "None"))
  (if (< (Math|Vector|VectorLengthSquared _returnvalue_2) 1e+02)
    (Audio|PlaySoundatLocation "/Game/SciFiWeapLight/Sound/RocketLauncher/RL_Explosion_Cue.RL_Explosion_Cue" _returnvalue "0, 0, 0" 1.0 1.0 0.0 0 0 0)
    (Effects|SpawnEmitteratLocation "/Game/SciFiWeapLight/FX/Particles/P_RocketLauncher_Explosion_Dark.P_RocketLauncher_Explosion_Dark" _returnvalue)
    (Class|GameplayStatics|ApplyRadialDamagewithFalloff 3e+02 0.0 _returnvalue 0.0 1e+03 1.0 0 0 0 0 "ECC_Visibility")
    (Actor|DestroyActor)))

(fn ConstructionScript)