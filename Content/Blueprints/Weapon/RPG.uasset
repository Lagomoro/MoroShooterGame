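; RPG weapon Blueprint that handles the effects and projectile launch when the rocket launcher fires.
; When MakeFireEffectBP receives a true Fired flag, it plays the weapon body's fire animation and a world camera shake at that location.
; It then spawns a BulletRPG at the fire arrow and launches it forward by directly setting the rocket mesh's physics linear velocity.
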(event EventBeginPlay)

(event Collision|EventActorBeginOverlap
  (params (OtherActor :type Actor%20Object%20Reference)))

(event EventTick
  (params (DeltaSeconds :type Float%20%28single-precision%29)))

(event EventMakeFireEffectBP
  (params (Fired :type Boolean))
  (bind _weaponfirearrow (Variables|Default|GetWeaponFireArrow))
  (if Fired
    (Components|Animation|PlayAnimation (Variables|Default|GetWeaponBody) "/Game/SciFiWeapLight/Weapons/Anims/Fire_RocketLauncher_W.Fire_RocketLauncher_W" false)
    (Camera|PlayWorldCameraShake "/Game/Blueprints/MoroCameraShake.MoroCameraShake_C" (Transformation|GetWorldLocation (Variables|Default|GetWeaponBody)) 0.0 5e+02 3.0)
    (bind _returnvalue (Game|SpawnActorfromClass "/Game/Blueprints/Weapon/BulletRPG.BulletRPG_C" (Transformation|GetWorldTransform _weaponfirearrow) "AdjustIfPossibleButAlwaysSpawn" 0 0))
    (Class|PrimitiveComponent|SetAllPhysicsLinearVelocity (Variables|/Game/Blueprints/Weapon/BulletRPG.BulletRPG_C|GetWhite_RocketLauncher_Ammo _returnvalue) (* (Math|Vector|GetForwardVector _weaponfirearrow) 10000) false)))

(fn ConstructionScript)