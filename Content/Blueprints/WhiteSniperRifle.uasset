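; White sniper rifle weapon Blueprint that supplies the cosmetic fire and hit effects through events taking a fired flag or hit data.
; Firing plays the weapon animation, launches a WhiteSniperRifleEffect actor from the fire arrow by setting physics velocity, and shakes nearby cameras.
; After a delay it destroys only that effect's root component, not the actor.
; Hits spawn a sound and particle from GetHitEffect, which returns the same pair for every physical material.
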(event EventBeginPlay
  (|CallParentFunction))

(event Collision|EventActorBeginOverlap
  (params (OtherActor :type Actor%20Object%20Reference))
  (|CallParentFunction OtherActor))

(event EventMakeFireEffectBP
  (params (Fired :type Boolean))
  (bind _weaponfirearrow (Variables|Default|GetWeaponFireArrow))
  (if Fired
    (Components|Animation|PlayAnimation (Variables|Default|GetWeaponBody) "/Game/SciFiWeapLight/Weapons/Anims/Fire_SniperRifle_W.Fire_SniperRifle_W" false)
    (bind _returnvalue (Game|SpawnActorfromClass "/Game/Blueprints/WhiteSniperRifleEffect.WhiteSniperRifleEffect_C" (Transformation|GetWorldTransform _weaponfirearrow) "Undefined" 0 0))
    (Class|PrimitiveComponent|SetAllPhysicsLinearVelocity (Variables|/Game/Blueprints/WhiteSniperRifleEffect.WhiteSniperRifleEffect_C|GetBase _returnvalue) (* (Math|Vector|GetForwardVector _weaponfirearrow) 40000) false)
    (Camera|PlayWorldCameraShake "/Game/Blueprints/MoroCameraShake.MoroCameraShake_C" (Transformation|GetWorldLocation (Variables|Default|GetWeaponBody)) 0.0 5e+02 3.0)
    (Utilities|FlowControl|Delay 5.0)
    (Components|DestroyComponent (Variables|/Script/Engine.Actor|GetRootComponent _returnvalue))))

(event EventTick
  (params (DeltaSeconds :type Float%20%28single-precision%29)))

(event EventMakeHitEffectBP
  (params (HitPhysicalMaterial :type Physical%20Material%20Object%20Reference) (HitLocation :type Vector :default "0, 0, 0") (HitActor :type Actor%20Object%20Reference) (HitComponent :type Primitive%20Component%20Object%20Reference) (HitBoneName :type Name :default "None"))
  (bind (_partical _sound) (CallFunction|GetHitEffect HitPhysicalMaterial))
  (Audio|PlaySoundatLocation _sound HitLocation "0, 0, 0" 1.0 1.0 0.0 0 0 0)
  (Effects|SpawnEmitteratLocation _partical HitLocation))

(fn ConstructionScript)

(fn GetHitEffect
  (params (Material :type Object%20Object%20Reference))
  (return "/Game/InfinityBladeEffects/Effects/FX_Mobile/combat/P_Shout_00.P_Shout_00" "/Game/SciFiWeapLight/Sound/SniperRifle/SR_ImpactSurface_Cue.SR_ImpactSurface_Cue"))