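; Player character Blueprint that handles death, scoring, respawn and hit feedback on top of events from its parent class.
; On server death it increments a valid instigator's MyPlayerState score, then after a short delay asks MyGameMode to respawn the player.
; Client hit confirmation finds the MyHUD widget and plays its hit effect.
; Death-on-all and kill-confirm handlers look up the HUD and player state but display nothing, and Tick is empty.
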(event EventBeginPlay
  (|CallParentFunction))

(event Collision|EventActorBeginOverlap
  (params (OtherActor :type Actor%20Object%20Reference)))

(event EventActionDieBPonAll
  (params (EventInstigator :type Pawn%20Object%20Reference) (DamageCauser :type Actor%20Object%20Reference))
  (if (Pawn|IsLocallyControlled)
    (bind _foundwidgets (Widget|GetAllWidgetsOfClass "/Game/Blueprints/Widgets/MyHUD.MyHUD_C" true))
    (Utilities|IsValid DamageCauser
      (:Is%20Valid
        (bind _asmy_player_state (Utilities|Casting|CastToMyPlayerState (Variables|/Script/Engine.Pawn|GetPlayerState EventInstigator)))))))

(event EventOnConfirmedKillBPonClient
  (params (KilledPawn :type Pawn%20Object%20Reference))
  (bind _foundwidgets (Widget|GetAllWidgetsOfClass "/Game/Blueprints/Widgets/MyHUD.MyHUD_C" true))
  (bind _asmy_player_state (Utilities|Casting|CastToMyPlayerState (Variables|/Script/Engine.Pawn|GetPlayerState KilledPawn))))

(event EventOnConfirmedHitBPonClient
  (params (HitPawn :type Pawn%20Object%20Reference))
  (bind _foundwidgets (Widget|GetAllWidgetsOfClass "/Game/Blueprints/Widgets/MyHUD.MyHUD_C" true))
  (Default|ShowHitEffect (Utilities|Array|Get(acopy) _foundwidgets)))

(event EventTick
  (params (DeltaSeconds :type Float%20%28single-precision%29))
  (if (Pawn|IsLocallyControlled)
    _))

(event EventTakeDamageBP
  (params (DamageAmount :type Float%20%28single-precision%29) (EventInstigator :type Controller%20Object%20Reference) (DamageCauser :type Actor%20Object%20Reference)))

(event EventActionDieBPonServer
  (params (EventInstigator :type Pawn%20Object%20Reference) (DamageCauser :type Actor%20Object%20Reference))
  (Utilities|IsValid EventInstigator
    (:Is%20Valid
      (bind _asmy_player_state (Utilities|Casting|CastToMyPlayerState (Variables|/Script/Engine.Pawn|GetPlayerState EventInstigator)))
      (Default|IncrementScore _asmy_player_state 1))
    (:Is%20Not%20Valid
      _))
  (Utilities|FlowControl|Delay 3.0)
  (bind _asmy_game_mode (Utilities|Casting|CastToMyGameMode (Game|GetGameMode)))
  (bind _as玩家控制器 (Utilities|Casting|CastToPlayerController (Pawn|GetController)))
  (Default|RespawnPlayerEvent _asmy_game_mode _as玩家控制器))

(fn ConstructionScript)